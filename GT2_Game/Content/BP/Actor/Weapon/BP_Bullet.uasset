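; Bullet actor that damages enemies on contact.
; Overlap events on a sphere and a capsule collision component run identical logic: cast the other actor to BP_Enemy, directly subtract a fixed amount from its AIHeath, then destroy the bullet.
; Overlaps with other actor types are ignored, and the graphs contain no movement logic.
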(event `self.CollisonSphere.OnComponentBeginOverlap`
  (params (OverlappedComponent :type "PrimitiveComponent Object Reference") (OtherActor :type "Actor Object Reference") (OtherComp :type "PrimitiveComponent Object Reference") (OtherBodyIndex :type Integer) (bFromSweep :type Boolean) (SweepResult :type "HitResult Structure (by ref)"))
  ;[1 1 1] Damage to enemy and destroy
  (bind _asbp_enemy (cast `/Game/BP/Character/BP_Enemy` OtherActor))
  (set `/Game/BP/Character/BP_Enemy.AIHeath` (- (`/Game/BP/Character/BP_Enemy.AIHeath` _asbp_enemy) 1.0) _asbp_enemy)
  (`self.K2_DestroyActor`))

(event `self.Capsule-collison.OnComponentBeginOverlap`
  (params (OverlappedComponent :type "PrimitiveComponent Object Reference") (OtherActor :type "Actor Object Reference") (OtherComp :type "PrimitiveComponent Object Reference") (OtherBodyIndex :type Integer) (bFromSweep :type Boolean) (SweepResult :type "HitResult Structure (by ref)"))
  ;[1 1 1] Damage to enemy and destroy
  (bind _asbp_enemy (cast `/Game/BP/Character/BP_Enemy` OtherActor))
  (set `/Game/BP/Character/BP_Enemy.AIHeath` (- (`/Game/BP/Character/BP_Enemy.AIHeath` _asbp_enemy) 1.0) _asbp_enemy)
  (`self.K2_DestroyActor`))

(fn `UserConstructionScript`)